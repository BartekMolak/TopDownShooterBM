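; Player-controlled marine soldier with world-axis movement, a HUD widget created on BeginPlay, and clamped health that sets Dead at zero.
; Each Tick, when mouse velocity exceeds a dead zone, control rotation interpolates toward the yaw of the mouse's movement direction.
; Fire input toggles the rifle muzzle-flash particles and firing sound, with an end sound on release; no hit or projectile logic is present.
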(event Game|Damage|EventAnyDamage
  (params (Damage :type Float%20%28single-precision%29) (DamageType :type Damage%20Type%20Object%20Reference) (InstigatedBy :type Controller%20Object%20Reference) (DamageCauser :type Actor%20Object%20Reference))
  (bind _output_get (Variables|Character|SetHealth (Math|Float|Clamp(Float) (- (Variables|Character|GetHealth) Damage) 0.0 1e+02)))
  (Variables|Default|SetDead (== _output_get 0.0)))

(event Collision|EventActorBeginOverlap
  (params (OtherActor :type Actor%20Object%20Reference)))

(event EventTick
  (params (DeltaSeconds :type Float%20%28single-precision%29))
  ;[1 1 1] Movement
  (CallFunction|UpdatePlayerRotation))

(event EventBeginPlay
  (bind _returnvalue (UserInterface|CreateWidget "/Game/UI/W_PlayerHUD.W_PlayerHUD_C" 0 self))
  (UserInterface|Viewport|AddtoViewport _returnvalue 0))

(event Input|ActionEvents|InputActionFireWeapon
  (params (Key :type Key%20Structure :default "None"))
  ;[1 1 1] Shooting gun
  (:Pressed
    (CallFunction|StartFiringWeapon))
  (:Released
    (CallFunction|StopFiringWeapon)))

(event Input|AxisEvents|InputAxisMoveForwardBack
  (params (AxisValue :type Float%20%28single-precision%29))
  ;[1 1 1] Movement
  (Pawn|Input|AddMovementInput "1.000000, 0, 0" AxisValue false))

(event Input|AxisEvents|InputAxisMoveLeftRight
  (params (AxisValue :type Float%20%28single-precision%29))
  ;[1 1 1] Movement
  (Pawn|Input|AddMovementInput "0.000000,1.000000, 0" AxisValue false))

(fn ConstructionScript)

(fn GetMouseVelocity
  (bind _returnvalue (Game|GetPlayerController 0))
  (bind (_deltax _deltay) (Class|PlayerController|GetInputMouseDelta _returnvalue))
  (return (/ (Math|Vector2D|MakeVector2D _deltax _deltay) (Utilities|Time|GetWorldDeltaSeconds))))

(fn UpdatePlayerRotation
  (bind _returnvalue (Game|GetPlayerController 0))
  (bind _returnvalue_2 (CallFunction|GetMouseVelocity))
  (if (CallFunction|IsMouseDeadZone)
    (Pawn|SetControlRotation _returnvalue (Math|Interpolation|RInterpTo (Transformation|GetActorRotation _returnvalue) (Math|Rotator|MakeRotator 0.0 0.0 (Class|KismetMathLibrary|DegAtan2 (.x _returnvalue_2) (.y _returnvalue_2))) (Utilities|Time|GetWorldDeltaSeconds) (Variables|Default|GetDeltaTimeMultiply)))))

(fn IsMouseDeadZone
  (return (> (Math|Vector2D|Vector2DLength (CallFunction|GetMouseVelocity)) (Variables|Default|GetMouseDeadZone))))

(fn StartFiringWeapon
  (Components|Activation|Activate (Variables|Default|GetP_AssaultRifle_MF) false)
  (bind _returnvalue (Audio|SpawnSound2D "/Game/Sounds/Weapon_AssaultRifle/Stereo/AssaultRifleShootStereoCue.AssaultRifleShootStereoCue" 1.0 1.0 0.0 0))
  (Variables|Default|SetWeaponFiring _returnvalue))

(fn StopFiringWeapon
  (Components|Activation|Deactivate (Variables|Default|GetP_AssaultRifle_MF))
  (Audio|Components|Audio|Stop (Variables|Default|GetWeaponFiring))
  (Audio|SpawnSound2D "/Game/Sounds/Weapon_AssaultRifle/Stereo/GunFireEnd.GunFireEnd" 1.0 1.0 0.0 0))